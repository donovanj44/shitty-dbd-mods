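; Actor that, despite its shadow map name, provides hotkey overrides for the local player's camera.
; Tick polls the first player controller for F8, which disables aspect ratio constraint and sets a square ratio, or F7, which widens the field of view.
; Each override casts the player character to both Slasher and Camper classes and edits that class's camera.
; Nothing in its graphs touches lighting or shadows, or reverts the changes.
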(event EventTick
  (params (DeltaSeconds :type Float%20%28single-precision%29))
  (if (Game|Player|WasInputKeyJustPressed (Game|GetPlayerController 0) "F8")
    (Utilities|FlowControl|Sequence
      (:then_0
        (bind _asbp_slasher_character (Utilities|Casting|CastToBP_Slasher_Character (Game|GetPlayerCharacter 0)))
        (Class|CameraComponent|SetConstraintAspectRatio (Variables|/Game/Characters/Slashers/Blueprints/BP_Slasher_Character.BP_Slasher_Character_C|GetCamera1 _asbp_slasher_character) false)
        (Class|CameraComponent|SetAspectRatio (Variables|/Game/Characters/Slashers/Blueprints/BP_Slasher_Character.BP_Slasher_Character_C|GetCamera1 _asbp_slasher_character) 1.0))
      (:then_1
        (bind _asbp_camper_character (Utilities|Casting|CastToBP_Camper_Character (Game|GetPlayerCharacter 0)))
        (Class|CameraComponent|SetConstraintAspectRatio (Variables|/Game/Characters/Campers/Blueprints/BP_Camper_Character.BP_Camper_Character_C|GetStraightCam _asbp_camper_character) false)
        (Class|CameraComponent|SetAspectRatio (Variables|/Game/Characters/Campers/Blueprints/BP_Camper_Character.BP_Camper_Character_C|GetStraightCam _asbp_camper_character) 1.0)))
    (elif (Game|Player|WasInputKeyJustPressed (Game|GetPlayerController 0) "F7")
      (Utilities|FlowControl|Sequence
        (:then_0
          (bind _asbp_slasher_character_2 (Utilities|Casting|CastToBP_Slasher_Character (Game|GetPlayerCharacter 0)))
          (Camera|SetFieldOfView (Variables|/Game/Characters/Slashers/Blueprints/BP_Slasher_Character.BP_Slasher_Character_C|GetCamera1 _asbp_slasher_character_2) 115.0))
        (:then_1
          (bind _asbp_camper_character_2 (Utilities|Casting|CastToBP_Camper_Character (Game|GetPlayerCharacter 0)))
          (Camera|SetFieldOfView (Variables|/Game/Characters/Campers/Blueprints/BP_Camper_Character.BP_Camper_Character_C|GetStraightCam _asbp_camper_character_2) 115.0))))))

(fn ConstructionScript)