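; Joke "freek" perk that harasses the player with random meme sounds and Among Us-themed screen overlays.
; Tick drives a chain of random Delays that plays an announcer "Skill Issue" clip and a Vine boom, then shows one of four widgets on player 0's viewport for a few seconds.
; Tick also sets a looping random-interval timer every frame on the FunnyPerk event, which is empty.
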(event Custom|funny%20perk)

(event EventBeginPlay)

(event EventTick
  (params (DeltaSeconds :type Float%20%28single-precision%29))
  (bind _returnvalue (Math|Random|RandomIntegerinRange 2 10))
  (bind _returnvalue_2 (Math|Random|RandomFloatinRange 0.0 15.0))
  (bind _returnvalue_3 (Game|GetPlayerController 0))
  (bind _returnvalue_4 (Math|Conversions|ToFloat(Integer) _returnvalue))
  (Utilities|Time|SetTimerbyEvent (delegate Custom|funny%20perk) (Math|Random|RandomFloatinRange 0.0 2e+01) true)
  (Utilities|FlowControl|Delay _returnvalue_2)
  (Audio|PlaySound2D "/Game/Blueprint/Perks/freekperk_assets/Halo_Announcer_says_Skill_Issue.Halo_Announcer_says_Skill_Issue" 2.0 1.0 0.0 0 0)
  (Utilities|FlowControl|Delay _returnvalue_2)
  (Audio|PlaySound2D "/Game/Blueprint/Perks/freekperk_assets/Vine_Boom_Sound_Effect.Vine_Boom_Sound_Effect" 1.0 1.0 0.0 0 0)
  (switch int (Math|Random|RandomIntegerinRange 0 3)
    (:0
      (bind _returnvalue_5 (UserInterface|CreateWidget "/Game/Blueprint/Perks/freekperk_assets/amogus_widget.amogus_widget_C" _returnvalue_3))
      (UserInterface|Viewport|AddtoViewport _returnvalue_5 0)
      (Utilities|FlowControl|Delay _returnvalue_4)
      (Widget|RemovefromParent _returnvalue_5))
    (:1
      (bind _returnvalue_6 (UserInterface|CreateWidget "/Game/Blueprint/Perks/freekperk_assets/among_us_drip_widget.among_us_drip_widget_C" _returnvalue_3))
      (UserInterface|Viewport|AddtoViewport _returnvalue_6 0)
      (Utilities|FlowControl|Delay _returnvalue_4)
      (Widget|RemovefromParent _returnvalue_6))
    (:2
      (bind _returnvalue_7 (UserInterface|CreateWidget "/Game/Blueprint/Perks/freekperk_assets/im_amogus_widget.im_amogus_widget_C" _returnvalue_3))
      (UserInterface|Viewport|AddtoViewport _returnvalue_7 0)
      (Utilities|FlowControl|Delay _returnvalue_4)
      (Widget|RemovefromParent _returnvalue_7))
    (:3
      (bind _returnvalue_8 (UserInterface|CreateWidget "/Game/Blueprint/Perks/freekperk_assets/pokemonamogus_widget.pokemonamogus_widget_C" _returnvalue_3))
      (UserInterface|Viewport|AddtoViewport _returnvalue_8 0)
      (Utilities|FlowControl|Delay _returnvalue_4)
      (Widget|RemovefromParent _returnvalue_8))))