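; Game instance for Horologium that bootstraps its core UI and offers shared spawn and lobby-widget events.
; On Init, after a short delay, it adds the core widget to the viewport if absent and plays a quiet test applause sound.
; Other events show a single slasher info widget for the lobby and remove it via a stored reference.
; A spawn helper creates any actor class at a given transform, owned by the DBD player character.
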(event EventInit
  (Utilities|FlowControl|Delay 1.0)
  (Utilities|FlowControl|Sequence
    (:then_0
      (bind _foundwidgets (Widget|GetAllWidgetsOfClass "/Game/Horologium/Blueprints/Widgets/WBP_HorologiumCore.WBP_HorologiumCore_C" true))
      (if (< (Utilities|Array|Length _foundwidgets) 1)
        (bind _returnvalue (UserInterface|CreateWidget "/Game/Horologium/Blueprints/Widgets/WBP_HorologiumCore.WBP_HorologiumCore_C" (Class|DBDGameInstance|GetLocalPlayerController)))
        (UserInterface|Viewport|AddtoViewport _returnvalue 0)))
    (:then_1
      (Audio|PlaySound2D "/Game/Horologium/Sounds/SFX/Testing_Applause.Testing_Applause" 0.05 1.0 0.0 0 0))))

(event EventSpawnActorfromClass
  (params (Actor%20Class :type Actor%20Class%20Reference) (Actor%20Location :type Vector :default "0, 0, 0") (Actor%20Rotation :type Rotator :default "0, 0, 0") (Actor%20Scale :type Vector :default "0, 0, 0"))
  (Game|SpawnActorfromClass Actor%20Class (Math|Transform|MakeTransform Actor%20Location Actor%20Rotation Actor%20Scale) "Undefined" (.DBDPlayerReference (CallFunction|FSGMGetDBDPlayerCharacter)) 0))

(event EventShowLobbyKIllerInfo
  (bind _foundwidgets (Widget|GetAllWidgetsOfClass "/Game/Horologium/Blueprints/Widgets/WBP_HorologiumSlasherInfo.WBP_HorologiumSlasherInfo_C" true))
  (if (== (Utilities|Array|Length _foundwidgets) 0)
    (bind _returnvalue (UserInterface|CreateWidget "/Game/Horologium/Blueprints/Widgets/WBP_HorologiumSlasherInfo.WBP_HorologiumSlasherInfo_C"))
    (bind _output_get (Variables|References|SetWBP%20Menu%20Killer%20Info%20Reference _returnvalue))
    (UserInterface|Viewport|AddtoViewport _output_get 0)))

(event EventDestroyLobbyKillerInfo
  (Widget|RemovefromParent (Variables|References|GetWBP%20Menu%20Killer%20Info%20Reference)))