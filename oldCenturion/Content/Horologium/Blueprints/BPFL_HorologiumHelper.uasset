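; Blueprint function library of helpers for Horologium, querying and manipulating a Dead by Daylight match.
; Getters wrap game state and instance to build maps of killers, survivors, generators, totems, traps and exit gates, translating engine states into simplified structs, enums or flags.
; Other helpers run camera line traces, snap (teleport) or immobilize the local character, and detect lobby versus gameplay.
; Data tables supply friendly character names and drive destroy-and-respawn lighting swaps.
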(fn FSGMSnapCharacterbyLineTrace
  (params (SnapDistance :type Float%20%28single-precision%29) (HeightDecrease :type Float%20%28single-precision%29))
  (bind _endposition (LineTrace|FSGMLineTraceEndPosition SnapDistance))
  (Class|DBDPlayer|SnapCharacter (.DBDPlayerReference (Reference|FSGMGetDBDPlayerCharacter)) true (Math|Vector|MakeVector (.x _endposition) (.y _endposition) (/ (.z _endposition) HeightDecrease)) 0.0 false "0, 0, 0" 0.0 false false false))

(fn FSGMGetIteminHands
  (return (Class|CharacterInventoryComponent|GetItem (Class|DBDPlayer|GetCharacterInventoryComponent (Class|DBDUtilities|GetLocallyControlledCharacter)))))

(fn FSGMGetItemName
  (params (CollectableObject :type Collectable%20Object%20Reference))
  (bind _returnvalue (Utilities|String|ToString(Object) CollectableObject))
  (if (Utilities|Array|IsEmpty _returnvalue)
    (return "{EMPTY}")
    (else
      (return _returnvalue))))

(fn FSGMGetSurvivorsAliveArray
  (bind _returnvalue (Class|DBDUtilities|GetDBDGameInstance))
  (bind _outplayingsurvivors (Class|DBDGameInstance|GetinGameAliveSurvivors _returnvalue))
  (return _outplayingsurvivors (Utilities|Array|Length _outplayingsurvivors)))

(fn FSGMGetSurvivorsArray
  (bind _returnvalue (Class|DBDUtilities|GetDBDGameInstance))
  (bind _returnvalue_2 (Class|DBDGameInstance|GetinGameSurvivors _returnvalue))
  (return _returnvalue_2 (Utilities|Array|Length _returnvalue_2)))

(fn FSGMGetSlashersArray
  (bind _returnvalue (Class|DBDUtilities|GetDBDGameInstance))
  (bind _returnvalue_2 (Class|DBDGameInstance|GetinGameKillers _returnvalue))
  (return _returnvalue_2 (Utilities|Array|Length _returnvalue_2)))

(fn FSGMGetPlayersArray
  (bind _returnvalue (Class|DBDUtilities|GetDBDGameInstance))
  (bind _returnvalue_2 (Class|DBDGameInstance|GetinGameKillers _returnvalue))
  (return _returnvalue_2 (Utilities|Array|Length _returnvalue_2)))

(fn FSGMGetDBDPlayerCharacter
  (bind _returnvalue (Class|DBDUtilities|GetDBDGameMode))
  (bind _returnvalue_2 (Class|DBDUtilities|GetLocallyControlledCharacter _returnvalue))
  (return _returnvalue_2 (Class|DBDPlayer|GetPlayerRole _returnvalue_2)))

(fn FSGMGetDBDPlayerCharacterasRole
  (if (Class|DBDUtilities|IsinSurvivorTeam)
    (return (Class|DBDUtilities|GetLocallyControlledSurvivor))
    (else
      (return (Class|DBDUtilities|GetLocallyControlledKiller)))))

(fn FSGMGetAllSlashersMap
  (for _array_element (Class|DBDGameInstance|GetinGameKillers (Class|DBDUtilities|GetDBDGameInstance))
    (bind _returnvalue (Class|CharacterInventoryComponent|GetAddons (Class|DBDPlayer|GetCharacterInventoryComponent _array_element)))
    (Utilities|Map|Add (LocalVariables|GetTEMP_OUTPUT) _array_element (Utilities|Struct|MakeS_SlasherInfo (.FriendlyName (String|FSGMGetDBDPlayerFriendlyName _array_element)) (Class|CharacterInventoryComponent|GetItem (Class|DBDPlayer|GetCharacterInventoryComponent _array_element)) _returnvalue)))
  (return (LocalVariables|GetTEMP_OUTPUT)))

(fn FSGMGetAllSlashersButMeMap
  (bind _slashersmap (MapValue|FSGMGetAllSlashersMap))
  (bind _output_get (LocalVariables|SetTEMP_OUTPUT _slashersmap))
  (Utilities|Map|Remove _slashersmap (Class|DBDUtilities|GetLocallyControlledKiller))
  (return _output_get))

(fn FSGMGetSlasherMeMap
  (bind _returnvalue (Class|DBDUtilities|GetLocallyControlledKiller))
  (return (Utilities|Map|MakeMap _returnvalue (.Value (Utilities|Map|Find (MapValue|FSGMGetAllSlashersMap) _returnvalue)))))

(fn FSGMGetAllSurvivorsMap
  (for _array_element (Class|DBDGameInstance|GetinGameSurvivors (Class|DBDUtilities|GetDBDGameInstance))
    (LocalVariables|SetTEMP_SURVIVORHEALTH "NewEnumerator0")
    (LocalVariables|SetTEMP_SURVIVORSTATE "NewEnumerator0")
    (switch string (Utilities|String|EnumtoString (Class|CamperHealthComponent|GetDamageState (Class|CamperPlayer|GetHealthComponent _array_element)))
      (:VE_Healthy
        (LocalVariables|SetTEMP_SURVIVORHEALTH "NewEnumerator1"))
      (:VE_Injured
        (LocalVariables|SetTEMP_SURVIVORHEALTH "NewEnumerator2"))
      (:VE_KO
        (LocalVariables|SetTEMP_SURVIVORHEALTH "NewEnumerator3"))
      (:VE_Dead
        (LocalVariables|SetTEMP_SURVIVORHEALTH "NewEnumerator4")))
    (if (Class|CamperPlayer|IsImmobilized _array_element)
      (switch string (Utilities|String|EnumtoString (Class|CamperPlayer|GetImmobilizedState _array_element))
        (:VE_Hiding
          (LocalVariables|SetTEMP_SURVIVORSTATE "NewEnumerator1"))
        (:VE_Trapped
          (LocalVariables|SetTEMP_SURVIVORSTATE "NewEnumerator2"))
        (:VE_Hooked
          (LocalVariables|SetTEMP_SURVIVORSTATE "NewEnumerator2")))
      (else
        (LocalVariables|SetTEMP_SURVIVORSTATE "NewEnumerator4")
        (switch Utilities|FlowControl|Switch|SwitchonECamperGuidedAction (Class|CamperPlayer|GetGuidedAction _array_element)
          (:VE_None
            _)
          (:VE_PrepBeingKilled
            _)
          (:VE_BeingKilled
            _)
          (:VE_PrepGuidedAction
            _)
          (:VE_BeingHelpedOffHookFront
            _)
          (:VE_BeingHelpedOffHookBack
            _)
          (:VE_BeingPickedUp
            _)
          (:VE_BeingPutDown
            _)
          (:VE_BeingCarried
            _)
          (:VE_BeingPutOnHook
            _)
          (:VE_BeingHealed
            (LocalVariables|SetTEMP_SURVIVORSTATE "NewEnumerator5"))
          (:VE_BeingPulledFromCloset
            _)
          (:VE_BeingHelpedFromTrap
            _)
          (:VE_AttachReverseBearTrap
            _)
          (:VE_BeingMended
            (LocalVariables|SetTEMP_SURVIVORSTATE "NewEnumerator6"))
          (:VE_BeingInjectedWithSerum
            _))
        (bind _returnvalue (Class|CharacterInventoryComponent|GetAddons (Class|DBDPlayer|GetCharacterInventoryComponent _array_element)))
        (Utilities|Map|Add (LocalVariables|GetTEMP_OUTPUT) _array_element (Utilities|Struct|MakeS_SurvivorInfo (.FriendlyName (String|FSGMGetDBDPlayerFriendlyName _array_element)) (LocalVariables|GetTEMP_SURVIVORHEALTH) (LocalVariables|GetTEMP_SURVIVORSTATE) (Class|CharacterInventoryComponent|GetItem (Class|DBDPlayer|GetCharacterInventoryComponent _array_element)) _returnvalue)))))
  (return (LocalVariables|GetTEMP_OUTPUT)))

(fn FSGMGetAllSurvivorsButMeMap
  (bind _output_get (LocalVariables|SetTEMP_OUTPUT (MapValue|FSGMGetAllSurvivorsMap)))
  (Utilities|Map|Remove _output_get (Class|DBDUtilities|GetLocallyControlledSurvivor))
  (return _output_get))

(fn FSGMGetSurvivorMeMap
  (bind _returnvalue (Class|DBDUtilities|GetLocallyControlledSurvivor))
  (return (Utilities|Map|MakeMap _returnvalue (.Value (Utilities|Map|Find (MapValue|FSGMGetAllSurvivorsMap) _returnvalue)))))

(fn FSGMGetGeneratorsMap
  (bind _temp_genstatedefine (LocalVariables|GetTEMP_GENSTATEDEFINE))
  (bind _output (Utilities|Array|Get(acopy) _temp_genstatedefine 5))
  (bind _output_2 (Utilities|Array|Get(acopy) _temp_genstatedefine 1))
  (bind _output_3 (Utilities|Array|Get(acopy) _temp_genstatedefine 2))
  (bind _output_4 (Utilities|Array|Get(acopy) _temp_genstatedefine 3))
  (bind _output_5 (Utilities|Array|Get(acopy) _temp_genstatedefine 4))
  (for _array_element (Class|DBDGameState|GetinGameGenerators (Reference|FSGMGetDBDGameState))
    (LocalVariables|SetTEMP_GENSTATE "NewEnumerator0")
    (LocalVariables|SetTEMP_GENSTATUS "NewEnumerator0")
    (LocalVariables|SetTEMP_GENCHARGEPERCENT (* (Class|Generator|GetChargePercentComplete _array_element) 1e+02))
    (if (Class|Generator|IsBlocked _array_element)
      (LocalVariables|SetTEMP_GENSTATUS "NewEnumerator2")
      (elif (Class|Generator|IsRegressing _array_element)
        (LocalVariables|SetTEMP_GENSTATUS "NewEnumerator1")
        (elif (Class|Generator|IsBeingRepaired _array_element)
          (LocalVariables|SetTEMP_GENSTATUS "NewEnumerator3"))))
    (Utilities|FlowControl|Sequence
      (:then_0
        (if (<= (LocalVariables|GetTEMP_GENCHARGEPERCENT) 0.0)
          (LocalVariables|SetTEMP_GENSTATE "NewEnumerator1")
          (Utilities|Map|Add (LocalVariables|GetTEMP_OUTPUT) _array_element (Utilities|Struct|MakeS_GeneratorInfo (LocalVariables|GetTEMP_GENSTATE) (LocalVariables|GetTEMP_GENSTATUS) "NewEnumerator0" (LocalVariables|GetTEMP_GENCHARGEPERCENT)) :!label _label)))
      (:then_1
        (if (Math|Float|InRange(Float) (LocalVariables|GetTEMP_GENCHARGEPERCENT) (Utilities|Array|Get(acopy) _temp_genstatedefine) _output_2 false false)
          (LocalVariables|SetTEMP_GENSTATE "NewEnumerator2")
          (goto _label)))
      (:then_2
        (if (Math|Float|InRange(Float) (LocalVariables|GetTEMP_GENCHARGEPERCENT) _output_2 _output_3 true false)
          (LocalVariables|SetTEMP_GENSTATE "NewEnumerator6")
          (goto _label)))
      (:then_3
        (if (Math|Float|InRange(Float) (LocalVariables|GetTEMP_GENCHARGEPERCENT) _output_3 _output_4 true false)
          (LocalVariables|SetTEMP_GENSTATE "NewEnumerator3")
          (goto _label)))
      (:then_4
        (if (Math|Float|InRange(Float) (LocalVariables|GetTEMP_GENCHARGEPERCENT) _output_4 _output_5 true false)
          (LocalVariables|SetTEMP_GENSTATE "NewEnumerator7")
          (goto _label)))
      (:then_5
        (if (Math|Float|InRange(Float) (LocalVariables|GetTEMP_GENCHARGEPERCENT) _output_5 _output true false)
          (LocalVariables|SetTEMP_GENSTATE "NewEnumerator4")
          (goto _label)))
      (:then_6
        (if (>= (LocalVariables|GetTEMP_GENCHARGEPERCENT) _output)
          (LocalVariables|SetTEMP_GENSTATE "NewEnumerator5")
          (goto _label)))))
  (return (LocalVariables|GetTEMP_OUTPUT)))

(fn FSGMGetTotemsMap
  (bind _outactors (Actor|GetAllActorsOfClass 0 "/Script/DeadByDaylight.Totem"))
  (for _array_element _outactors
    (LocalVariables|SetTEMP_TOTEMSTATE "NewEnumerator0")
    (switch Utilities|FlowControl|Switch|SwitchonETotemState (Class|Totem|GetTotemState _array_element)
      (:Cleansed
        (bind _output_get (LocalVariables|SetTEMP_TOTEMSTATE "NewEnumerator4")))
      (:Dull
        (LocalVariables|SetTEMP_TOTEMSTATE "NewEnumerator1"))
      (:Hex
        (LocalVariables|SetTEMP_TOTEMSTATE "NewEnumerator2"))
      (:Boon
        (LocalVariables|SetTEMP_TOTEMSTATE "NewEnumerator3")))
    (Utilities|Map|Add (LocalVariables|GetTEMP_OUTPUT) _array_element _output_get))
  (return (LocalVariables|GetTEMP_OUTPUT)))

(fn FSGMGetTrapsMap
  (for _array_element (Class|DBDGameState|GetinGameBaseTraps (Reference|FSGMGetDBDGameState))
    (if (not (Utilities|String|StartsWith (Utilities|String|ToString(Object) _array_element) "BP_" "CaseSensitive"))
      (Utilities|Map|Add (LocalVariables|GetTEMP_OUTPUT) _array_element (Class|BaseTrap|IsTrapSet _array_element))))
  (return (LocalVariables|GetTEMP_OUTPUT)))

(fn FSGMGetExitGatesMap
  (for _array_element (Class|DBDGameState|GetinGameEscapeDoors (Reference|FSGMGetDBDGameState))
    (LocalVariables|SetTEMP_ESCAPEDOORSTATE "NewEnumerator1")
    (Utilities|FlowControl|Sequence
      (:then_0
        (if (Class|EscapeDoor|IsActivated _array_element)
          (if (Class|EscapeDoor|GetIsOpen _array_element)
            (LocalVariables|SetTEMP_ESCAPEDOORSTATE "NewEnumerator3")
            (else
              (LocalVariables|SetTEMP_ESCAPEDOORSTATE "NewEnumerator2")))))
      (:then_1
        (if (Class|EscapeDoor|IsDoorSwitchBlocked _array_element)
          (LocalVariables|SetTEMP_ESCAPEDOORSTATE "NewEnumerator5"))
        (Utilities|Map|Add (LocalVariables|GetTEMP_OUTPUT) _array_element (LocalVariables|GetTEMP_ESCAPEDOORSTATE)))))
  (return (LocalVariables|GetTEMP_OUTPUT)))

(fn FSGMLineTraceActor
  (params (Distance :type Float%20%28single-precision%29))
  (bind _dbdplayerreference (Reference|FSGMGetDBDPlayerCharacter))
  (bind _returnvalue (Class|DBDPlayer|GetCameraManager _dbdplayerreference))
  (bind _returnvalue_2 (Camera|GetCameraLocation _returnvalue))
  (bind _outhit (Collision|LineTraceByChannel 0 _returnvalue_2 (+ _returnvalue_2 (* (Math|Vector|GetForwardVector (Camera|GetCameraRotation _returnvalue)) Distance)) "TraceTypeQuery1" false (Utilities|Array|MakeArray _dbdplayerreference) "None"))
  (return (.hitactor _outhit)))

(fn FSGMLineTraceHitPosition
  (params (Distance :type Float%20%28single-precision%29))
  (bind _dbdplayerreference (Reference|FSGMGetDBDPlayerCharacter))
  (bind _returnvalue (Class|DBDPlayer|GetCameraManager _dbdplayerreference))
  (bind _returnvalue_2 (Camera|GetCameraLocation _returnvalue))
  (bind _outhit (Collision|LineTraceByChannel 0 _returnvalue_2 (+ _returnvalue_2 (* (Math|Vector|GetForwardVector (Camera|GetCameraRotation _returnvalue)) Distance)) "TraceTypeQuery1" false (Utilities|Array|MakeArray _dbdplayerreference) "None"))
  (return (.location _outhit)))

(fn FSGMLineTraceEndPosition
  (params (Distance :type Float%20%28single-precision%29))
  (bind _dbdplayerreference (Reference|FSGMGetDBDPlayerCharacter))
  (bind _returnvalue (Class|DBDPlayer|GetCameraManager _dbdplayerreference))
  (bind _returnvalue_2 (Camera|GetCameraLocation _returnvalue))
  (bind _outhit (Collision|LineTraceByChannel 0 _returnvalue_2 (+ _returnvalue_2 (* (Math|Vector|GetForwardVector (Camera|GetCameraRotation _returnvalue)) Distance)) "TraceTypeQuery1" false (Utilities|Array|MakeArray _dbdplayerreference) "None"))
  (return (.traceend _outhit)))

(fn FSGMGetDBDPlayerFriendlyName
  (params (DBDPlayer :type DBD%20Player%20Object%20Reference))
  (bind _returnvalue (Class|DBDBasePlayer|GetCharacterName DBDPlayer))
  (bind _returnvalue_2 (Utilities|GetDataTableRow "/Game/Horologium/Blueprints/Data/DT_DBDCharacters.DT_DBDCharacters" _returnvalue)
    (:then
      (return (.dbdcharactername _returnvalue_2) (.dbdplayerrole _returnvalue_2)))
    (:RowNotFound
      (return (Utilities|String|ToString(Name) _returnvalue) "NewEnumerator0"))))

(fn FSGMGetCurrentLevel
  (bind _returnvalue (Game|GetCurrentLevelName 0))
  (Utilities|IsValid (Class|DBDUtilities|GetLocallyControlledCharacter)
    (:Is%20Valid
      (return _returnvalue "NewEnumerator2"))
    (:Is%20Not%20Valid
      (return _returnvalue "NewEnumerator1"))))

(fn FSGMGetIsinGameplayLevel
  (switch Utilities|FlowControl|Switch|SwitchonE_LevelType (.E_LevelType (AdvancedInfo|FSGMGetCurrentLevel))
    (:NewEnumerator0
      _)
    (:NewEnumerator1
      _)
    (:NewEnumerator2
      (return true)))
  (return false))

(fn FSGMGetDBDGameState
  (return (Class|DBDUtilities|GetDBDGameState (Game|GetGameState))))

(fn FSGMGetSlasherItem
  (params (SlasherPlayerReference :type Slasher%20Player%20Object%20Reference))
  (return (Class|CharacterInventoryComponent|GetItem (Class|DBDPlayer|GetCharacterInventoryComponent SlasherPlayerReference))))

(fn FSGMGetDBDGameInstance
  (return (Class|DBDUtilities|GetDBDGameInstance (Class|CoreUtilities|GetGameInstance))))

(fn FSGMGetDBDBasePlayerFriendlyName
  (params (DBDBasePlayer :type DBD%20Base%20Player%20Object%20Reference))
  (bind _returnvalue (Class|DBDBasePlayer|GetCharacterName DBDBasePlayer))
  (bind _returnvalue_2 (Utilities|GetDataTableRow "/Game/Horologium/Blueprints/Data/DT_DBDCharacters.DT_DBDCharacters" _returnvalue)
    (:then
      (return (.dbdcharactername _returnvalue_2) (.dbdplayerrole _returnvalue_2)))
    (:RowNotFound
      (return (Utilities|String|ToString(Name) _returnvalue) "NewEnumerator0"))))

(fn FSGMSnapCharacterbyLocationwithRotation
  (params (Target%20Location :type Vector) (Final%20Character%20Rotation :type Rotator))
  (Class|DBDPlayer|SnapCharacter (.DBDPlayerReference (Reference|FSGMGetDBDPlayerCharacter)) true Target%20Location 0.0 false Final%20Character%20Rotation 0.0 false false false))

(fn FSGMSnapCharacterbyLocation
  (params (Target%20Location :type Vector) (Keep%20Character%20Rotation? :type Boolean))
  (bind _dbdplayerreference (Reference|FSGMGetDBDPlayerCharacter))
  (if Keep%20Character%20Rotation?
    (Class|DBDPlayer|SnapCharacter _dbdplayerreference true Target%20Location 0.0 false (Transformation|GetActorRotation _dbdplayerreference) 0.0 false false false)
    (else
      (Class|DBDPlayer|SnapCharacter _dbdplayerreference true Target%20Location 0.0 false "0, 0, 0" 0.0 false false false))))

(fn FSGMDestroyLightingonMap
  (bind _outrownames (DataTable|GetDataTableRowNames "/Game/Horologium/Blueprints/Data/DT_DBDLighting.DT_DBDLighting"))
  (for _array_element _outrownames
    (bind _returnvalue (Utilities|GetDataTableRow "/Game/Horologium/Blueprints/Data/DT_DBDLighting.DT_DBDLighting" _array_element)
      (:then
        (bind _outactors (Actor|GetAllActorsOfClass 0 (.lightingobjectclass _returnvalue)))
        (for _array_element_2 _outactors
          (Actor|DestroyActor _array_element_2))))))

(fn FSGMSwapLightingonMap
  (params (New%20Lighting :type Name))
  (Function|FSGMDestroyLightingonMap)
  (bind _returnvalue (Utilities|GetDataTableRow "/Game/Horologium/Blueprints/Data/DT_DBDLighting.DT_DBDLighting" New%20Lighting)
    (:then
      (Class|BPIHorologiumGameInstance|SpawnActorfromClass(Message) (Reference|FSGMGetDBDGameInstance) (.lightingobjectclass _returnvalue) "0, 0, 0" "0, 0, 0" "1.000000,1.000000,1.000000"))))

(fn FSGMSetSelfImmobilized
  (params (ImmobilizedState :type ECamperImmobilizeState%20Enum :default "VE_None"))
  (Class|CamperPlayer|SetImmobilized (Class|DBDUtilities|GetLocallyControlledSurvivor (.DBDPlayerReference (Reference|FSGMGetDBDPlayerCharacter))) ImmobilizedState))

(fn FSGMGetDBDPlayerFriendlyNamebyCharacterID
  (params (CharacterID :type Integer))
  (bind _outrownames (DataTable|GetDataTableRowNames "/Game/Horologium/Blueprints/Data/DT_DBDCharacters.DT_DBDCharacters"))
  (for _array_element _outrownames
    (bind _returnvalue (Utilities|GetDataTableRow "/Game/Horologium/Blueprints/Data/DT_DBDCharacters.DT_DBDCharacters" _array_element)
      (:then
        (if (== (.DBDCharacterId (Utilities|Struct|BreakS_DBDCharacters _returnvalue)) CharacterID)
          (return (.DBDCharacterName (Utilities|Struct|BreakS_DBDCharacters _returnvalue)) (.DBDPlayerRole (Utilities|Struct|BreakS_DBDCharacters _returnvalue)))))))
  (return "UNKNOWN" "NewEnumerator0"))